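; BP_Hider is the playable hider character, with Enhanced Input movement and look plus pallet dropping and vaulting.
; Interact takes the first overlapping BP_Pallet, skips it if destroyed, forces rotation to its snap transform, then asks the server to run the pallet's DoInteract.
; Multicast events play drop and vault montages between start and stop state calls.
; Vaulting also lerps actor location along a timeline scaled to VaultTime, without sweeping.
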(event `EnhancedInput|/Game/ThirdPerson/Input/Actions/IA_Move`
  (params (ActionValue :type "Vector2D Structure") (ElapsedSeconds :type "Float (double-precision)") (TriggeredSeconds :type "Float (double-precision)") (InputAction :type "InputAction Object Reference" :default "/Game/ThirdPerson/Input/Actions/IA_Move.IA_Move"))
  (bind _returnvalue (`KismetMathLibrary.MakeRotator` 0.0 0.0 (.yaw (`self.GetControlRotation`))))
  (:`Triggered`
    (`self.AddMovementInput` (`KismetMathLibrary.GetRightVector` _returnvalue) ActionValue_X)
    (`self.AddMovementInput` (`KismetMathLibrary.GetForwardVector` _returnvalue) ActionValue_Y)))

(event `EnhancedInput|/Game/ThirdPerson/Input/Actions/IA_Look`
  (params (ActionValue :type "Vector2D Structure") (ElapsedSeconds :type "Float (double-precision)") (TriggeredSeconds :type "Float (double-precision)") (InputAction :type "InputAction Object Reference" :default "/Game/ThirdPerson/Input/Actions/IA_Look.IA_Look"))
  (:`Triggered`
    (`self.AddControllerYawInput` ActionValue_X)
    (`self.AddControllerPitchInput` ActionValue_Y)))

(event `self.ReceiveBeginPlay`
  (`EnhancedInputSubsystemInterface.AddMappingContext` (pcsubsystem `EnhancedInputLocalPlayerSubsystem` (`GameplayStatics.GetPlayerController` 0)) "/Game/ThirdPerson/Input/IMC_Default.IMC_Default" 0 (struct)))

(event `self.ReceiveActorBeginOverlap`
  (params (OtherActor :type "Actor Object Reference")))

(event `self.ReceiveTick`
  (params (DeltaSeconds :type "Float (single-precision)")))

(event `EnhancedInput|/Game/ThirdPerson/Input/Actions/IA_Interaction`
  (params (ActionValue :type Boolean) (ElapsedSeconds :type "Float (double-precision)") (TriggeredSeconds :type "Float (double-precision)") (InputAction :type "InputAction Object Reference" :default "/Game/ThirdPerson/Input/Actions/IA_Interaction.IA_Interaction"))
  (bind _overlappingactors (`self.GetOverlappingActors` self "/Game/Asset/Blueprints/MapObject/BP_Pallet.BP_Pallet_C"))
  (bind _output (`|GetArrayItem` _overlappingactors))
  ; Pallet Interact
  (:`Started`
    (if (> (`KismetArrayLibrary.Array_Length` _overlappingactors) 0)
      (if (`|EnumInequality` (`Pallet.PalletState` _output) "Destroyed")
        (bind _returnvalue (`Pallet.GetSnapTransform` _output self))
        (`self.SetForceRotation` true (.rotation _returnvalue))
        (`self.Server_HiderRequestInteract` _output)))))

(event `Server_HiderRequestInteract`
  (params (TargetPallet :type "/Game/Asset/Blueprints/MapObject/BP_Pallet Object Reference"))
  ; Pallet Interact
  (`Pallet.DoInteract` TargetPallet self))

(event `Multicast_PalletDrop`
  ; Multicast Pallet Drop
  (`self.StartPalletDrop`)
  (`|PlayMontage` (`self.Mesh`) "/Game/Asset/Animation/Anim_DropPallet.Anim_DropPallet"
    (:`OnCompleted`
      _)
    (:`OnInterrupted`
      _))
  (`self.StopPalletDrop`))

(event `Multicast_PalletVault`
  (params (VaultStartLoc :type "Vector Structure") (VaultEndLoc :type "Vector Structure"))
  ; Multicast Pallet Vault
  (`self.StartVaulting`)
  (`|ExecutionSequence`
    (:`then_0`
      (`|PlayMontage` (`self.Mesh`) "/Game/Asset/Animation/Anim_PalletVault.Anim_PalletVault"
        (:`OnCompleted`
          _)
        (:`OnInterrupted`
          _))
      (`self.StopVaulting`))
    (:`then_1`
      (`TimelineComponent.SetPlayRate` (`self.VaultTimeline`) (/ 1.0 (`self.VaultTime`)))
      (bind (_direction _alpha) (`Timeline|VaultTimeline` :!via `PlayFromStart`)
        (:`Update`
          (`self.K2_SetActorLocation` (`KismetMathLibrary.VLerp` VaultStartLoc VaultEndLoc _alpha)))))))

(fn `UserConstructionScript`)