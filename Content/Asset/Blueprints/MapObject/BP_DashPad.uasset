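; BP_DashPad is a one-use map pad that, once a hider activates it, launches tagged Hiders and Seekers along its arrow at role-specific speeds.
; Activation dashes current overlaps, and TriggerBox catches new ones, toggling ignore-move-input around each launch.
; Inside the overlap loop, it also recolors the pad via server-to-multicast events and, after a delay, expires it and disables interaction collision.
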(event `self.BP_OnHiderInteractDashPad`
  (params (Hider :type "Actor Object Reference"))
  (set `self.bIsActive` true)
  (for _array_element (`PrimitiveComponent.GetOverlappingActors` (`self.TriggerBox`) "/Script/Engine.Actor")
    (`self.ExcuteDash` _array_element)
    (`self.Server_ChangePadColor` (`KismetMathLibrary.Conv_LinearColorToVector` (`KismetMathLibrary.MakeColor` 1.0 1.0)))
    (`KismetSystemLibrary.Delay` 2.0)
    (set `self.bIsActive` false)
    (set `self.bIsExpired` true)
    (`self.Server_ChangePadColor` (`KismetMathLibrary.Conv_LinearColorToVector` (`KismetMathLibrary.MakeColor` 0.0)))
    (`PrimitiveComponent.SetCollisionEnabled` (`self.InteractionBox`) "NoCollision")))

(event `Server_ChangePadColor`
  (params (Color :type "Vector Structure"))
  (`self.Multicast_ChangeColor` Color))

(event `Multicast_ChangeColor`
  (params (Color :type "Vector Structure"))
  (`MeshComponent.SetVectorParameterValueOnMaterials` (`self.StaticMesh`) "Color" Color))

(event `self.TriggerBox.OnComponentBeginOverlap`
  (params (OverlappedComponent :type "PrimitiveComponent Object Reference") (OtherActor :type "Actor Object Reference") (OtherComp :type "PrimitiveComponent Object Reference") (OtherBodyIndex :type Integer) (bFromSweep :type Boolean) (SweepResult :type "HitResult Structure (by ref)"))
  (`self.ExcuteDash` OtherActor))

(event `ExcuteDash`
  (params (TargetActor :type "Actor Object Reference"))
  ; ExcuteDash
  (if (`self.bIsActive`)
    (if (`self.ActorHasTag` TargetActor "Hider")
      (bind _ascharacter (cast `Character` TargetActor))
      (bind _returnvalue (`Pawn.GetController` _ascharacter))
      (`Controller.SetIgnoreMoveInput` _returnvalue false)
      (`Character.LaunchCharacter` _ascharacter (+ (* (`SceneComponent.GetForwardVector` (`self.DirectionArrow`)) (`self.HiderSpeed`)) (0.0 0.0 200.0)) true true)
      (`KismetSystemLibrary.Delay` (`self.DisableTime`))
      (`Controller.SetIgnoreMoveInput` _returnvalue true)
      (elif (`self.ActorHasTag` TargetActor "Seeker")
        (bind _ascharacter_2 (cast `Character` TargetActor))
        (bind _returnvalue_2 (`Pawn.GetController` _ascharacter_2))
        (`Controller.SetIgnoreMoveInput` _returnvalue_2 false)
        (`Character.LaunchCharacter` _ascharacter_2 (+ (* (`SceneComponent.GetForwardVector` (`self.DirectionArrow`)) (`self.SeekerSpeed`)) (0.0 0.0 200.0)) true true)
        (`KismetSystemLibrary.Delay` (`self.DisableTime`))
        (`Controller.SetIgnoreMoveInput` _returnvalue_2 true)))))

(fn `UserConstructionScript`)