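; BP_Pallet is a map-object pallet that hiders drop and vault, and that stuns seekers or gets destroyed by them.
; On drop, a timeline lerps the mesh from its initial relative transform, applied at BeginPlay, to a lowered, tilted pose.
; Drop, vault, stun and destroy events cast to BP_Hider or BP_Seeker and delegate to that character's multicast or server functions.
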(event `self.ReceiveBeginPlay`
  (`SceneComponent.K2_SetRelativeLocationAndRotation` (`self.PalletMesh`) (`self.InitMeshRelativeLocation`) (`self.InitMeshRelativeRotation`) false false))

(event `self.BP_OnPalletDropped`
  ; OnPalletDropped
  (bind (_direction _alpha) (`Timeline|Timeline` :!via `PlayFromStart`)
    (:`Update`
      (`SceneComponent.K2_SetRelativeLocationAndRotation` (`self.PalletMesh`) (`KismetMathLibrary.VLerp` (`self.InitMeshRelativeLocation`) (0.0 0.0 -30.0) _alpha) (`KismetMathLibrary.RLerp` (`self.InitMeshRelativeRotation`) (struct :`Roll` 60.0) _alpha) false false))))

(event `self.BP_OnHiderDropPallet`
  (params (Hider :type "Actor Object Reference"))
  ; OnPalletDropped
  (bind _asbp_hider (cast `/Game/Asset/Blueprints/Character/BP_Hider` Hider))
  (`/Game/Asset/Blueprints/Character/BP_Hider.Multicast_PalletDrop` _asbp_hider))

(event `self.BP_OnHiderVault`
  (params (Hider :type "Actor Object Reference") (StartLoc :type "Vector Structure") (EndLoc :type "Vector Structure"))
  ; OnHiderVault
  (bind _asbp_hider (cast `/Game/Asset/Blueprints/Character/BP_Hider` Hider))
  (`/Game/Asset/Blueprints/Character/BP_Hider.Multicast_PalletVault` _asbp_hider StartLoc EndLoc))

(event `self.BP_OnSeekerStunned`
  (params (Seeker :type "Actor Object Reference") (StunTime :type "Float (single-precision)"))
  ; SeekerStun
  (bind _asbp_seeker (cast `/Game/Asset/Blueprints/Character/BP_Seeker` Seeker))
  (`SeekerCharacter.Server_ApplyStun` _asbp_seeker StunTime))

(event `self.BP_OnSeekerDestroyPallet`
  (params (Seeker :type "Actor Object Reference"))
  (bind _asbp_seeker (cast `/Game/Asset/Blueprints/Character/BP_Seeker` Seeker))
  (`/Game/Asset/Blueprints/Character/BP_Seeker.Multicast_PalletDestroy` _asbp_seeker self))

(fn `UserConstructionScript`)